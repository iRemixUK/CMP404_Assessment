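; Behavior tree task that sends a BP_Enemy running toward the castle.
; On execute, it takes the run location from the BP_PlaceableActor found in the level and sets the enemy's movement velocity to that direction times Speed.
; It writes velocity directly rather than using pathfinding, then finishes successfully right away.
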(event `self.ReceiveExecuteAI`
  (params (OwnerController :type "AIController Object Reference") (ControlledPawn :type "Pawn Object Reference"))
  ;[1 1 1] Get enemy character movement
  (bind _output_get (set `self.Controlled Pawn` ControlledPawn))
  (bind _asbp_enemy (cast `/Game/Blueprints/Enemy/BP_Enemy` _output_get))
  (set `self.Character Movement` (`Character.CharacterMovement` _asbp_enemy))
  ;[1 1 1] Get the location for the enemy to run to then get the unit direction multiplied by speed and set the velocity of the enemy so that they can run to the castle
  (bind _returnvalue (`GameplayStatics.GetActorOfClass` "/Game/Blueprints/BP_PlaceableActor.BP_PlaceableActor_C"))
  (set `MovementComponent.Velocity` (* (`KismetMathLibrary.GetDirectionUnitVector` (`Actor.K2_GetActorLocation` (`self.Controlled Pawn`)) (`/Game/Blueprints/BP_PlaceableActor.LocationToRun` _returnvalue)) (`self.Speed`)) (`self.Character Movement`))
  (`self.FinishExecute` true))