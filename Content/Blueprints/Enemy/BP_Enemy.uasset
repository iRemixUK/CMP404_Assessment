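; Enemy actor that runs a behavior tree and shows its health, in a game built around a placeable castle.
; On BeginPlay it starts BT_AIRunTo and takes its scale from BP_PlaceableActor's PlaceableScale.
; Each tick it pushes Health to the health bar widget and copies the placeable actor's rotation to face the castle.
; While Health is zero or below, it replays the death sound every tick, with no destroy logic here.
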(event `self.ReceiveBeginPlay`
  ;[1 1 1] Run behaviour tree
  (`AIController.RunBehaviorTree` (`AIBlueprintHelperLibrary.GetAIController` self) "/Game/Blueprints/Enemy/BT_AIRunTo.BT_AIRunTo")
  ;[1 1 1] Set actor scale
  (bind _returnvalue (`GameplayStatics.GetActorOfClass` "/Game/Blueprints/BP_PlaceableActor.BP_PlaceableActor_C"))
  (`self.SetActorScale3D` (`PlaceableActor.PlaceableScale` _returnvalue)))

(event `self.ReceiveTick`
  (params (DeltaSeconds :type "Float (single-precision)"))
  ;[1 1 1] Set health bar's health value
  (bind _aswbp_enemy_health_bar (cast `/Game/Blueprints/UserInterface/WBP_EnemyHealthBar` (`WidgetComponent.GetWidget` (`self.HealthBar`))))
  (set `/Game/Blueprints/UserInterface/WBP_EnemyHealthBar.CurrentHealth` (`self.Health`) _aswbp_enemy_health_bar)
  ;[1 1 1] Set actor rotation so that it is always facing the castle
  (bind _returnvalue (`GameplayStatics.GetActorOfClass` "/Game/Blueprints/BP_PlaceableActor.BP_PlaceableActor_C"))
  (`self.K2_SetActorRotation` (`self.K2_GetActorRotation` _returnvalue))
  ;[1 1 1] Play death sound if enemy is dead
  (if (<= (`self.Health`) 0.0)
    (`GameplayStatics.PlaySound2D` "/Game/Assets/Audio/DeathSound.DeathSound" 1.0 1.0 0.0 null null)))

(fn `UserConstructionScript`)