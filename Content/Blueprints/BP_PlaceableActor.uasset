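; BP_PlaceableActor is the player's placeable castle, which enemies attack from three child-actor spawners.
; SetChildActors activates the spawners and starts the music, while Tick keeps their scale matched to the castle and refreshes LocationToRun from the Box position.
; An enemy overlapping the Box damages the castle, increments the game mode's defeated count and is destroyed.
; At zero health it pauses the game, stops the music, shows the end screen and destroys itself.
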(event `self.ReceiveBeginPlay`
  ;[1 1 1] Set location to run
  (set `self.LocationToRun` (`SceneComponent.K2_GetComponentLocation` (`self.Box`))))

(event `self.Box.OnComponentBeginOverlap`
  (params (OverlappedComponent :type "PrimitiveComponent Object Reference") (OtherActor :type "Actor Object Reference") (OtherComp :type "PrimitiveComponent Object Reference") (OtherBodyIndex :type Integer) (bFromSweep :type Boolean) (SweepResult :type "HitResult Structure (by ref)"))
  ;[1 1 1] If enemy reaches the castle destroy the enemy, take damage and increment enemies defeated
  (bind _asbp_enemy (cast `/Game/Blueprints/Enemy/BP_Enemy` OtherActor))
  (`self.TakeDamageFromEnemy`)
  (bind _asbp_custom_game_mode (cast `/Game/Blueprints/BP_CustomGameMode` (`GameplayStatics.GetGameMode`)))
  (`CustomGameMode.IncrementEnemiesDefeated` _asbp_custom_game_mode)
  (`self.K2_DestroyActor` _asbp_enemy))

(event `self.ReceiveTick`
  (params (DeltaSeconds :type "Float (single-precision)"))
  ;[1 1 1] Update location to run and set scale of the spawners
  (set `self.LocationToRun` (`SceneComponent.K2_GetComponentLocation` (`self.Box`)))
  (`SceneComponent.SetWorldScale3D` (`self.EnemySpawner_1`) (`self.GetActorScale3D`))
  (`SceneComponent.SetWorldScale3D` (`self.EnemySpawner_2`) (`self.GetActorScale3D`))
  (`SceneComponent.SetWorldScale3D` (`self.EnemySpawner_3`) (`self.GetActorScale3D`))
  ;[1 1 1] If health is less than or equal to zero the player has died and the end screen UI will be displayed. Once player has died stop playing game music
  (if (<= (`self.Health`) 0.0)
    (`GameplayStatics.SetGamePaused` true)
    (`ActorComponent.SetActive` (`self.GameMusic`) false false)
    (bind _returnvalue (`|CreateWidget` "/Game/Blueprints/UserInterface/WBP_EndScreen.WBP_EndScreen_C"))
    (`UserWidget.AddToViewport` _returnvalue 0)
    (`self.K2_DestroyActor`)))

(fn `SetChildActors`
  ;[1 1 1] Activates the spawners and sets location to run
  (set `self.LocationToRun` (+ (`SceneComponent.K2_GetComponentLocation` (`self.Box`)) (0.0 0.0 10.0)))
  (`ChildActorComponent.SetChildActorClass` (`self.EnemySpawner_1`) "/Game/Blueprints/Enemy/BP_EnemySpawner.BP_EnemySpawner_C")
  (`ChildActorComponent.SetChildActorClass` (`self.EnemySpawner_2`) "/Game/Blueprints/Enemy/BP_EnemySpawner.BP_EnemySpawner_C")
  (`ChildActorComponent.SetChildActorClass` (`self.EnemySpawner_3`) "/Game/Blueprints/Enemy/BP_EnemySpawner.BP_EnemySpawner_C")
  ;[1 1 1] Play music
  (bind _returnvalue (`GameplayStatics.SpawnSound2D` "/Game/Assets/Audio/GameMusic.GameMusic" 1.0 1.0 0.0 null))
  (set `self.GameMusic` _returnvalue))

(fn `UserConstructionScript`)